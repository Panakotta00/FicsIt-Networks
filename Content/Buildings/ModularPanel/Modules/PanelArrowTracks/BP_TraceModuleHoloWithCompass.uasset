(event `self.OnInputMappingBound`
  (params (Actions :type "Array of Name (by ref)"))
  (bind _mcachedkeybinds (`/Game/FactoryGame/Interface/UI/InGame/BuildMenu/Widget_BuildMode.mCachedKeybinds` (`self.BuildModeWidget`)))
  (`BlueprintLoggingLibrary.LogVerbose` "EVENT Input Mapping Bound")
  (if (> (`KismetArrayLibrary.Array_Length` Actions) 0)
    (bind _asbp_game_ui (cast `/Game/FactoryGame/Interface/UI/InGame/BP_GameUI` (`/Game/FactoryGame/Interface/UI/HUDHelpers/HUDHelpers.GetFGGameUI` (`GameplayStatics.GetPlayerController` 0))))
    (bind _widget (`/Game/FactoryGame/Interface/UI/HUDHelpers/BPHUDHelpers.FindWidgetOfClass` "/Game/FactoryGame/Interface/UI/InGame/BuildMenu/Widget_BuildMode.Widget_BuildMode_C" _asbp_game_ui))
    (`/Engine/EditorBlueprintResources/StandardMacros.IsValid` _widget
      (:`Is Valid`
        (bind _aswidget_build_mode (cast `/Game/FactoryGame/Interface/UI/InGame/BuildMenu/Widget_BuildMode` _widget)
          (:`then`
            (bind _output_get (set `self.BuildModeWidget` _aswidget_build_mode))
            (`KismetArrayLibrary.Array_AddUnique` _mcachedkeybinds (make `/Game/FactoryGame/Interface/UI/InGame/-Shared/KeybindingHints/Struct_KeybindingHint` "Configure" (`KismetTextLibrary.Conv_StringToText` (`KismetTextLibrary.Conv_TextToString` (`/Game/FactoryGame/Interface/UI/HUDHelpers/HUDHelpers.Get Key Name for Action Simple` (`GameplayStatics.GetPlayerController` 0) (`|GetArrayItem` Actions))))))
            (`/Game/FactoryGame/Interface/UI/InGame/BuildMenu/Widget_BuildMode.SetKeybindingHints` _output_get _mcachedkeybinds))
          (:`CastFailed`
            (`BlueprintLoggingLibrary.LogError` "Cast to Widget_BuildMode failed"))))
      (:`Is Not Valid`
        (`BlueprintLoggingLibrary.LogError` "Widget not found")))))

(event `self.OnInformationUpdate`
  (params (Component :type "TextRenderComponent Object Reference") (HitResult :type "HitResult Structure (by ref)") (SnappedPanel :type "FINModuleSystemPanel Object Reference") (ModuleLocation :type "Vector Structure") (ModuleRotation :type Integer))
  (bind _panelheight (`FINModuleSystemPanel.PanelHeight` SnappedPanel))
  (bind _panelwidth (`FINModuleSystemPanel.PanelWidth` SnappedPanel))
  (bind _returnvalue (`KismetStringLibrary.Conv_IntToString` (`KismetMathLibrary.FTrunc` (.y ModuleLocation))))
  (bind _returnvalue_2 (`KismetStringLibrary.Conv_IntToString` (`KismetMathLibrary.FTrunc` (.x ModuleLocation))))
  (cast `FINModuleBase` (`BlueprintReflectionLibrary.GetClassDefaultObject` (`self.GetBuildClass`))
    (:`then`
      (if (or (== _panelheight 1) (== _panelwidth 1))
        (if (> _panelheight _panelwidth)
          (set `self.TempText` (`KismetStringLibrary.Concat_StrStr` "X" _returnvalue_2))
          (else
            (set `self.TempText` (`KismetStringLibrary.Concat_StrStr` "X" _returnvalue))))
        (else
          (set `self.TempText` (`KismetStringLibrary.Concat_StrStr` "X" _returnvalue " Y" _returnvalue_2))))
      (`TextRenderComponent.K2_SetText` (`self.InformationComponent`) (`KismetTextLibrary.Conv_StringToText` (`self.TempText`))))
    (:`CastFailed`
      (`TextRenderComponent.K2_SetText` (`self.InformationComponent`) ":cerr:"))))

(fn `UserConstructionScript`)