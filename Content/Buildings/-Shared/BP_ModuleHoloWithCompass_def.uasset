(event `self.OnInformationUpdate`
  (params (Component :type "TextRenderComponent Object Reference") (HitResult :type "HitResult Structure (by ref)") (SnappedPanel :type "FINModuleSystemPanel Object Reference") (ModuleLocation :type "Vector Structure") (ModuleRotation :type Integer))
  (bind _panelwidth (`FINModuleSystemPanel.PanelWidth` SnappedPanel))
  (bind _panelheight (`FINModuleSystemPanel.PanelHeight` SnappedPanel))
  (bind _returnvalue (`KismetStringLibrary.Conv_IntToString` (`KismetMathLibrary.FTrunc` (.x ModuleLocation))))
  (bind _returnvalue_2 (`KismetStringLibrary.Conv_IntToString` (`KismetMathLibrary.FTrunc` (.y ModuleLocation))))
  (cast `FINModuleBase` (`BlueprintReflectionLibrary.GetClassDefaultObject` (`self.GetBuildClass`))
    (:`then`
      (if (or (== _panelheight 1) (== _panelwidth 1))
        (if (> _panelheight _panelwidth)
          (set `self.TempText` (`KismetStringLibrary.Concat_StrStr` "X" _returnvalue))
          (else
            (set `self.TempText` (`KismetStringLibrary.Concat_StrStr` "X" _returnvalue_2))))
        (else
          (set `self.TempText` (`KismetStringLibrary.Concat_StrStr` "X" _returnvalue_2 " Y" _returnvalue))))
      (`TextRenderComponent.K2_SetText` (`self.InformationComponent`) (`KismetTextLibrary.Conv_StringToText` (`self.TempText`))))
    (:`CastFailed`
      (`TextRenderComponent.K2_SetText` (`self.InformationComponent`) ":cerr:"))))

(fn `UserConstructionScript`)